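; Test player Blueprint for the menus that toggles the pause menu with a P debug key.
; The first press creates WBP_PauseMenu and caches it in PauseRef for reuse.
; Pausing shows the widget and cursor, switches to UI-only input and focuses the Resume button for keyboard use.
; The unpause branch removes the widget, hides the cursor and restores game-only input.
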(event Input|KeyboardEvents|DebugKeyP
  (params (Key :type Key%20Structure) (ActionValue :type Input%20Action%20Value%20Structure))
  (bind _returnvalue (Game|GetPlayerController 0))
  (bind _returnvalue_2 (Game|GetPlayerController 0))
  ;[0.3854 0.3854 0.3854] Pause
  (:Pressed
    (Utilities|IsValid (Variables|Default|GetPauseRef)
      (:Is%20Valid
        _)
      (:Is%20Not%20Valid
        (bind _returnvalue_3 (UserInterface|CreateWidget "/Game/Menus/Viewport/WBP_PauseMenu.WBP_PauseMenu_C"))
        (Variables|Default|SetPauseRef _returnvalue_3)))
    (if (Game|IsGamePaused)
      (Widget|RemovefromParent (Variables|Default|GetPauseRef))
      (Game|SetGamePaused false)
      (Variables|/Script/Engine.PlayerController|SetbShowMouseCursor _returnvalue_2 false)
      (Input|SetInputModeGameOnly _returnvalue_2 false)
      (else
        (UserInterface|Viewport|AddtoViewport (Variables|Default|GetPauseRef) 0)
        (Game|SetGamePaused true)
        (Variables|/Script/Engine.PlayerController|SetbShowMouseCursor _returnvalue true)
        (Input|SetInputModeUIOnly _returnvalue 0 "DoNotLock" false)
        (Widget|SetKeyboardFocus (Variables|/Game/Menus/Viewport/WBP_PauseMenu.WBP_PauseMenu_C|GetResumeButton (Variables|Default|GetPauseRef)))))))

(fn ConstructionScript)