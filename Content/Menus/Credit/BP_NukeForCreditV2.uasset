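; Nuke projectile for the credits menu that arcs toward a target location and explodes, occasionally swapping its mesh for a sausage.
; BeginPlay spawns a BP_Spline with a randomly offset, raised midpoint and scales the trajectory timeline's play rate by spline length.
; The timeline moves and orients the actor along the spline with sweep.
; Sphere overlap or timeline completion spawns an explosion field and nuclear VFX, then destroys the actor.
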(event `self.ReceiveBeginPlay`
  (bind _returnvalue (`self.K2_GetActorLocation`))
  (bind _sphere (`self.Sphere`))
  (bind _t_trajectory (`self.t_Trajectory`))
  (bind _returnvalue_2 (* (`KismetMathLibrary.Vector_Distance` (`self.K2_GetActorLocation`) (`self.targetLocation`)) (`KismetMathLibrary.RandomFloatInRange` 0.05 0.25)))
  ; Clacule trajectory
  (if (== (`KismetMathLibrary.RandomIntegerInRange` 0 10) 5)
    (`StaticMeshComponent.SetStaticMesh` _sphere "/Game/01_Meshes/Saucisson/SM_Saucisson_01.SM_Saucisson_01")
    (`PrimitiveComponent.SetMaterial` _sphere 0 "/Game/02_Materials/Props/MI_Saucisson_01.MI_Saucisson_01"))
  (bind _returnvalue_3 (`|SpawnActorFromClass` "/Game/Menus/Credit/BP_Spline.BP_Spline_C" (`KismetMathLibrary.MakeTransform` (`self.K2_GetActorLocation`) (`self.K2_GetActorRotation`)) "Undefined" "MultiplyWithRoot" null null))
  (set `self.splineActor` _returnvalue_3)
  (`SplineComponent.SetSplinePoints` (`/Game/Menus/Credit/BP_Spline.Spline` (`self.splineActor`)) (`|MakeArray` _returnvalue (+ (+ (* (- (`self.targetLocation`) _returnvalue) (`KismetMathLibrary.RandomFloatInRange` 0.3 0.7)) _returnvalue (* (`self.GetActorRightVector`) (`KismetMathLibrary.RandomFloatInRange` (* _returnvalue_2 -1.0) _returnvalue_2))) (`KismetMathLibrary.MakeVector` 0.0 0.0 _returnvalue_2)) (`self.targetLocation`)) "World" true)
  (bind _output_get (set `self.distance` (`SplineComponent.GetSplineLength` (`/Game/Menus/Credit/BP_Spline.Spline` (`self.splineActor`)))))
  (`TimelineComponent.SetPlayRate` _t_trajectory (/ 1.0 (`KismetMathLibrary.FClamp` (`KismetMathLibrary.MapRangeUnclamped` _output_get 0.0 100.0 0.0 0.2) 0.1)))
  (`TimelineComponent.PlayFromStart` _t_trajectory))

(event `Explosion`
  (bind _returnvalue (`self.K2_GetActorLocation`))
  ; Explose
  (`|SpawnActorFromClass` "/Game/Menus/Credit/BP_ExplosionField.BP_ExplosionField_C" (`KismetMathLibrary.MakeTransform` _returnvalue) "Undefined" "MultiplyWithRoot" null null :!label _label)
  (`/Game/BPFL_KiliLibrary.KL_SimpleVFX` "/Game/VFX/NS_SmallerNuclearBomb.NS_SmallerNuclearBomb" (`KismetMathLibrary.MakeTransform` _returnvalue))
  (`self.K2_DestroyActor`))

(event `self.Sphere.OnComponentBeginOverlap`
  (params (OverlappedComponent :type "PrimitiveComponent Object Reference") (OtherActor :type "Actor Object Reference") (OtherComp :type "PrimitiveComponent Object Reference") (OtherBodyIndex :type Integer) (bFromSweep :type Boolean) (SweepResult :type "HitResult Structure (by ref)"))
  ; Explose
  (goto _label))

(fn `UserConstructionScript`)