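; Player actor for the interactive credits screen, letting the player shoot nukes while the credits widget is displayed.
; On BeginPlay it adds WBP_Credit to the viewport and switches to game-only input.
; Shooting deprojects the mouse, traces along that ray and spawns BP_NukeForCreditV2 at the cursor's world position, targeting the impact or trace end.
; Aim input moves the mouse cursor by gamepad sensitivity, and the return input opens LVL_MenuTest.
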(event `self.ReceiveBeginPlay`
  (bind _returnvalue (`|CreateWidget` "/Game/Menus/Credit/WBP_Credit.WBP_Credit_C"))
  (`UserWidget.AddToViewport` _returnvalue 0)
  (`WidgetBlueprintLibrary.SetInputMode_GameOnly` (`GameplayStatics.GetPlayerController` 0)))

(event `EnhancedInput|/Game/Menus/Credit/Input/IA_Shoot`
  (params (ActionValue :type Boolean) (ElapsedSeconds :type "Float (double-precision)") (TriggeredSeconds :type "Float (double-precision)") (InputAction :type "InputAction Object Reference" :default "/Game/Menus/Credit/Input/IA_Shoot.IA_Shoot"))
  (bind (_worldlocation _worlddirection) (`PlayerController.DeprojectMousePositionToWorld` (`GameplayStatics.GetPlayerController` 0)))
  (:`Started`
    (bind (_outhit _returnvalue) (`KismetSystemLibrary.LineTraceSingle` _worldlocation (+ _worldlocation (* _worlddirection 5000.0)) "TraceTypeQuery1"))
    (bind (_bblockinghit _binitialoverlap _time _distance _location _impactpoint _normal _impactnormal _physmat _hitactor _hitcomponent _hitbonename _bonename _hititem _elementindex _faceindex _tracestart _traceend) (`GameplayStatics.BreakHitResult` _outhit))
    (`|SpawnActorFromClass` "/Game/Menus/Credit/BP_NukeForCreditV2.BP_NukeForCreditV2_C" (`KismetMathLibrary.MakeTransform` _worldlocation) "AdjustIfPossibleButAlwaysSpawn" "MultiplyWithRoot" null (`KismetMathLibrary.SelectVector` (`KismetMathLibrary.MakeVector` (.x _impactpoint) (.y _impactpoint) (.z _impactpoint)) _traceend _returnvalue) null)))

(event `EnhancedInput|/Game/Menus/Credit/Input/IA_ReturnToMenu`
  (params (ActionValue :type Boolean) (ElapsedSeconds :type "Float (double-precision)") (TriggeredSeconds :type "Float (double-precision)") (InputAction :type "InputAction Object Reference" :default "/Game/Menus/Credit/Input/IA_ReturnToMenu.IA_ReturnToMenu"))
  (:`Started`
    (`GameplayStatics.OpenLevelBySoftObjectPtr` "/Game/Menus/SceneMenus/LVL_MenuTest.LVL_MenuTest" false) ; Choose game scene
  ))

(event `EnhancedInput|/Game/Menus/Credit/Input/IA_AimCredit`
  (params (ActionValue :type "Vector2D Structure") (ElapsedSeconds :type "Float (double-precision)") (TriggeredSeconds :type "Float (double-precision)") (InputAction :type "InputAction Object Reference" :default "/Game/Menus/Credit/Input/IA_AimCredit.IA_AimCredit"))
  (bind (_x _y) (`KismetMathLibrary.BreakVector2D` ActionValue))
  (bind (_locationx _locationy) (`PlayerController.GetMousePosition` (`GameplayStatics.GetPlayerController` 0)))
  (bind (_x_2 _y_2) (`KismetMathLibrary.BreakVector2D` (+ (`KismetMathLibrary.MakeVector2D` _locationx _locationy) (* (`KismetMathLibrary.MakeVector2D` _x (* _y -1.0)) (`self.gamepadSensi`)))))
  (:`Triggered`
    (`PlayerController.SetMouseLocation` (`GameplayStatics.GetPlayerController` 0) (`KismetMathLibrary.FTrunc` _x_2) (`KismetMathLibrary.FTrunc` _y_2))))

(fn `UserConstructionScript`)