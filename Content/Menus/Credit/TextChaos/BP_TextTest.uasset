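; BP_TextTest is a credits text actor that scrolls along its up vector and returns the game to the menu level.
; Each Tick it uses VInterpTo toward a far point above its current location, giving a steady swept rise.
; Tick also feeds a two-minute Delay that then opens MenuLevel.
; A looping timer for the empty MoveCredit event is left unconnected and never runs.
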(event `self.ReceiveBeginPlay`)

(event `MoveCredit`)

(event `self.ReceiveTick`
  (params (DeltaSeconds :type "Float (single-precision)"))
  (bind _returnvalue (`self.K2_GetActorLocation`))
  (`self.K2_SetActorLocation` (`KismetMathLibrary.VInterpTo` _returnvalue (+ _returnvalue (* (`self.GetActorUpVector`) 10000.0)) (`GameplayStatics.GetWorldDeltaSeconds`) 0.05) true)
  (`KismetSystemLibrary.Delay` 120.0)
  (`GameplayStatics.OpenLevelBySoftObjectPtr` (`self.MenuLevel`) false) ; Choose game scene
)

(fn `UserConstructionScript`)