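; BP_TextGroup is an actor in the credits menu folder, apparently meant as a scrolling group of credit text, but none of its logic is wired up.
; BeginPlay, MoveCredit and the construction script are empty.
; Disconnected nodes hold the intended behavior: a looping timer for MoveCredit, an interpolated upward move along the actor's up vector, and a long delay before opening the menu level.
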(event `self.ReceiveBeginPlay`)

(event `MoveCredit`)

(fn `UserConstructionScript`)