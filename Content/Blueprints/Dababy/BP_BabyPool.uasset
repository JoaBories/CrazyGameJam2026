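; BP_BabyPool is an object pool for BP_LittleBaby actors.
; On BeginPlay it spawns babies in a loop up to BabyCount at its own transform, calls Retrieve on each and stores them in the Babies array.
; GetABaby scans the whole array without breaking and returns the last baby found that is not Activated, so existing actors can be reused.
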(event `self.ReceiveBeginPlay`
  (for _ (range (+ (`self.BabyCount`) 1))
    (bind _returnvalue (`|SpawnActorFromClass` "/Game/Blueprints/Dababy/BP_LittleBaby.BP_LittleBaby_C" (`self.GetTransform`) "AlwaysSpawn" "MultiplyWithRoot" null null))
    (`/Game/Blueprints/Dababy/BP_LittleBaby.Retrieve` _returnvalue)
    (`KismetArrayLibrary.Array_AddUnique` (`self.Babies`) _returnvalue)))

(fn `GetABaby`
  (returns (Baby :type "/Game/Blueprints/Dababy/BP_LittleBaby Object Reference"))
  (locals (Found :type "/Game/Blueprints/Dababy/BP_LittleBaby Object Reference"))
  (for _array_element (`self.Babies`)
    (if (not (`/Game/Blueprints/Dababy/BP_LittleBaby.Activated` _array_element))
      (set `local.Found` _array_element)))
  (return (`local.Found`)))

(fn `UserConstructionScript`)