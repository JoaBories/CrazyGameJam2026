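; BP_BabyCluster is a lobbed projectile that bursts into a group of pooled babies on landing.
; Shoot sets the target, flight time and count, then Tick moves it along a timer-driven sine arc, facing its motion.
; When the timer ends, it waits until the player's sphere is at least 50 units away.
; It then pulls babies from BP_BabyPool, spawns them in random directions around itself and destroys itself.
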(event `Shoot`
  (params (GoalPos :type "Vector Structure") (Time :type "Float (double-precision)") (Babies :type Integer))
  (bind _output_get (set `self.TotalTime` Time))
  (set `self.Time` _output_get)
  (set `self.Goal Pos` GoalPos)
  (set `self.StartPos` (`self.K2_GetActorLocation`))
  (set `self.Babies` Babies))

(event `self.ReceiveTick`
  (params (DeltaSeconds :type "Float (single-precision)"))
  (bind _returnvalue (`KismetMathLibrary.RandomFloat`))
  (bind _zero (`/Game/BPFL_KiliLibrary.KL_UpdateTimer` (`self.Time`) DeltaSeconds true))
  (if _zero
    (if (not (< (`KismetMathLibrary.Vector_DistanceSquared` (`SceneComponent.K2_GetComponentLocation` (`/Game/Blueprints/AAAAAAAAAAAAAAAA.Sphere` (cast `/Game/Blueprints/AAAAAAAAAAAAAAAA` (`GameplayStatics.GetPlayerPawn` 0) :!pure true))) (`self.K2_GetActorLocation`)) 2500.0))
      (bind _returnvalue_2 (`GameplayStatics.GetActorOfClass` "/Game/Blueprints/Dababy/BP_BabyPool.BP_BabyPool_C"))
      (for _ (range 1 (+ (`self.Babies`) 1))
        (bind _baby (`/Game/Blueprints/Dababy/BP_BabyPool.GetABaby` _returnvalue_2))
        (`/Engine/EditorBlueprintResources/StandardMacros.IsValid` _baby
          (:`Is Valid`
            (`/Game/Blueprints/Dababy/BP_LittleBaby.SpawnBaby` _baby (+ (* (`KismetMathLibrary.Normal2D` (`KismetMathLibrary.MakeVector2D` _returnvalue _returnvalue)) 100.0) (`self.K2_GetActorLocation`))))))
      (`self.K2_DestroyActor`))
    (else
      (bind _output_get (set `self.NextPos` (+ (* (`KismetMathLibrary.Sin` (* (/ (`self.Time`) (`self.TotalTime`)) (`KismetMathLibrary.GetPI`))) (`self.TotalTime`) 300.0 (`KismetMathLibrary.Vector_Up`)) (`|EaseFunction` "Linear" (/ (`self.Time`) (`self.TotalTime`)) (`self.Goal Pos`) (`self.StartPos`)))))
      (`self.K2_SetActorLocationAndRotation` _output_get (`KismetMathLibrary.FindLookAtRotation` (`self.K2_GetActorLocation`) _output_get)))))

(fn `UserConstructionScript`)