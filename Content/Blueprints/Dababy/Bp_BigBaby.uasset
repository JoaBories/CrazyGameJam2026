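; Big baby enemy character that chases the player and periodically lobs clusters of babies at them, tuned through a DataAsset.
; A looping timer re-issues AIMoveTo toward player 0 every 0.2 seconds.
; A second looping timer rolls a chance to fire a BP_BabyCluster at the player's current position.
; Flight time comes from 2D distance over cluster speed and also sets how long the Niagara warning at the target lasts.
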(event `self.ReceiveBeginPlay`
  (set `CharacterMovementComponent.MaxWalkSpeed` (`/Game/Blueprints/Dababy/DataAsset/BPDA_BigBaby.WalkingSpeed` (`self.DataAsset`)) (`self.CharacterMovement`))
  (`KismetSystemLibrary.K2_SetTimerDelegate` (delegate `BabyClusterTry`) (`/Game/BPFL_KiliLibrary.KL_1/x` (`/Game/Blueprints/Dababy/DataAsset/BPDA_BigBaby.BabyClusterFirerate` (`self.DataAsset`))) true)
  (set `self.Player` (`GameplayStatics.GetPlayerPawn` 0))
  (`KismetSystemLibrary.K2_SetTimerDelegate` (delegate `UpdateMovement`) 0.2 true))

(event `BabyClusterTry`
  (if (< (`KismetMathLibrary.RandomFloatInRange` 0.0 100.0) (`/Game/Blueprints/Dababy/DataAsset/BPDA_BigBaby.BabyClusterChance` (`self.DataAsset`)))
    (`self.LaunchBabies`)))

(event `UpdateMovement`
  (`|AIMoveTo` self (`self.K2_GetActorLocation` (`self.Player`)) null))

(fn `LaunchBabies`
  (locals (Time :type "Float (double-precision)") (Position :type "Vector Structure"))
  (set `local.Position` (`self.K2_GetActorLocation` (`GameplayStatics.GetPlayerPawn` 0)))
  (set `local.Time` (/ (`KismetMathLibrary.Vector_Distance2D` (`local.Position`) (`self.K2_GetActorLocation`)) (`/Game/Blueprints/Dababy/DataAsset/BPDA_BigBaby.BabyClusterSpeed` (`self.DataAsset`))))
  (bind _returnvalue (`/Game/BPFL_KiliLibrary.KL_SimpleVFX` "/Game/Blueprints/Dababy/Feedbacks/NS_ClusterWarning.NS_ClusterWarning" (`KismetMathLibrary.MakeTransform` (`self.K2_GetActorLocation` (`GameplayStatics.GetPlayerPawn` 0)))))
  (`NiagaraComponent.SetNiagaraVariableFloat` _returnvalue "Lasting" (`local.Time`))
  (bind _returnvalue_2 (`|SpawnActorFromClass` "/Game/Blueprints/Dababy/BP_BabyCluster.BP_BabyCluster_C" (`KismetMathLibrary.MakeTransform` (`self.K2_GetActorLocation`)) "AlwaysSpawn" "MultiplyWithRoot" null null))
  (`/Game/Blueprints/Dababy/BP_BabyCluster.Shoot` _returnvalue_2 (`local.Position`) (`local.Time`) (`/Game/Blueprints/Dababy/DataAsset/BPDA_BigBaby.BabiesNumber` (`self.DataAsset`))))

(fn `UserConstructionScript`)