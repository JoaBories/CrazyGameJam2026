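; BP_LittleBaby is a reusable character that chases the player's sphere and bursts into sparkles when it gets close.
; SpawnBaby places and activates it with a randomized walk speed, then a looping timer compares squared distances against data asset thresholds to AI-move or explode.
; Exploding and Die play VFX, then Retrieve hides it at its origin for reuse instead of destroying it.
; Slow scales or restores its walk speed.
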(event `self.ReceiveBeginPlay`
  (bind _asaaaaaaaaaaaaaaaa (cast `/Game/Blueprints/AAAAAAAAAAAAAAAA` (`GameplayStatics.GetPlayerPawn` 0)))
  (set `self.Player` (`/Game/Blueprints/AAAAAAAAAAAAAAAA.Sphere` _asaaaaaaaaaaaaaaaa))
  (set `self.Origin` (`self.K2_GetActorLocation`)))

(event `Retrieve`
  (`self.Activate` false)
  (`self.K2_SetActorLocation` (`self.Origin`))
  (set `MovementComponent.Velocity` (0.0 0.0 0.0) (`self.CharacterMovement`)))

(event `SpawnBaby`
  (params (Position :type "Vector Structure"))
  (bind _dataasset (`self.DataAsset`))
  (`self.K2_SetActorLocation` Position)
  (`ActorComponent.Activate` (`self.CharacterMovement`) true)
  (bind _output_get (set `self.BaseSpeed` (+ (`/Game/Blueprints/Dababy/DataAsset/BPDA_LittleBaby.WalkingSpeed` _dataasset) (* (`/Game/Blueprints/Dababy/DataAsset/BPDA_LittleBaby.WalkingVariance` _dataasset) (`KismetMathLibrary.RandomFloatInRange` -1.0 1.0)))))
  (set `CharacterMovementComponent.MaxWalkSpeed` _output_get (`self.CharacterMovement`))
  (`self.Activate` true)
  (bind _returnvalue (`KismetSystemLibrary.K2_SetTimerDelegate` (delegate `UpdateMovement`) (`/Game/BPFL_KiliLibrary.KL_1/x` (`/Game/Blueprints/Dababy/DataAsset/BPDA_LittleBaby.UpdateFrequency` (`self.DataAsset`))) true))
  (set `self.UpdateGoalTimer` _returnvalue))

(event `UpdateMovement`
  (bind (_explode _moveto) (`self.CheckDistances`))
  (if _explode
    (`/Game/BPFL_KiliLibrary.KL_SimpleVFX` "/Game/VFX/NS_SparkleBurst.NS_SparkleBurst" (`self.GetTransform`))
    (`self.Retrieve`)
    (elif _moveto
      (`|AIMoveTo` self (`SceneComponent.K2_GetComponentLocation` (`self.Player`)) null (`/Game/Blueprints/Dababy/DataAsset/BPDA_LittleBaby.AcceptanceRadius` (`self.DataAsset`))))))

(event `Slow`
  (params (Begin :type Boolean) (Amount :type "Float (double-precision)"))
  (bind _basespeed (`self.BaseSpeed`))
  (set `CharacterMovementComponent.MaxWalkSpeed` (`KismetMathLibrary.SelectFloat` (* _basespeed Amount) _basespeed Begin) (`self.CharacterMovement`)))

(event `Die`
  (`/Game/BPFL_KiliLibrary.KL_SimpleVFX` "/Game/VFX/NS_Splash.NS_Splash" (`self.GetTransform`))
  (`self.Retrieve`))

(fn `Activate`
  (params (Enable :type Boolean))
  (bind _output_get (set `self.Activated` Enable))
  (`SceneComponent.SetVisibility` (`self.Mesh`) _output_get true)
  (`self.SetActorEnableCollision` _output_get)
  (`self.SetActorTickEnabled` _output_get)
  (`KismetSystemLibrary.K2_ClearAndInvalidateTimerHandle` (`self.UpdateGoalTimer`)))

(fn `CheckDistances`
  (returns (Explode :type Boolean) (MoveTo :type Boolean))
  (locals (Distance :type "Float (double-precision)" :default 0.0))
  (bind _output_get (set `local.Distance` (`KismetMathLibrary.Vector_DistanceSquared` (`SceneComponent.K2_GetComponentLocation` (`self.Player`)) (`self.K2_GetActorLocation`))))
  (if (< _output_get (`KismetMathLibrary.MultiplyMultiply_FloatFloat` (`/Game/Blueprints/Dababy/DataAsset/BPDA_LittleBaby.DetectionDistance` (`self.DataAsset`)) 2.0))
    (return (< _output_get (`KismetMathLibrary.MultiplyMultiply_FloatFloat` (`/Game/Blueprints/Dababy/DataAsset/BPDA_LittleBaby.ExplodingDistance` (`self.DataAsset`)) 2.0)) true)
    (else
      (return false false))))

(fn `UserConstructionScript`)