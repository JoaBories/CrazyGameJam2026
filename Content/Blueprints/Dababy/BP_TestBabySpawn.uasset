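; BP_TestBabySpawn is a test spawner that places pooled babies at its own location on a repeating timer.
; On BeginPlay it finds the level's BP_BabyPool and starts a looping timer based on SpawnRate, or prints a warning if no pool exists.
; Each tick of the timer requests a baby from the pool and, if one is valid, spawns it at the spawner's position.
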(event `self.ReceiveBeginPlay`
  (bind _returnvalue (`GameplayStatics.GetActorOfClass` "/Game/Blueprints/Dababy/BP_BabyPool.BP_BabyPool_C"))
  (bind _output_get (set `self.Pool` _returnvalue))
  (`/Engine/EditorBlueprintResources/StandardMacros.IsValid` _output_get
    (:`Is Valid`
      (`KismetSystemLibrary.K2_SetTimerDelegate` (delegate `SpawnBaby`) (`/Game/BPFL_KiliLibrary.KL_1/x` (`self.SpawnRate`)) true))
    (:`Is Not Valid`
      (`KismetSystemLibrary.PrintString` "Missing Baby Pool In the level" true true (struct :`R` 1.0 :`B` 0.000247 :`A` 1.0) 10.0))))

(event `SpawnBaby`
  (bind _baby (`/Game/Blueprints/Dababy/BP_BabyPool.GetABaby` (`self.Pool`)))
  (`/Engine/EditorBlueprintResources/StandardMacros.IsValid` _baby
    (:`Is Valid`
      (`/Game/Blueprints/Dababy/BP_LittleBaby.SpawnBaby` _baby (`self.K2_GetActorLocation`)))))

(fn `UserConstructionScript`)