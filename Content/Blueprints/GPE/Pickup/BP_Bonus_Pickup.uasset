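; Respawning bonus pickup that grants its Pickup type to the player on overlap.
; The construction script picks the product mesh from that type and sizes the collision sphere from CollisionSize.
; Overlap by the first player's pawn passes the type to AddBonusPickup on an actor found by class, then plays a timeline scaling the mesh.
; When the timeline finishes, a cooldown hides and disables the pickup for a few seconds before restoring it.
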(event `self.ReceiveBeginPlay`
  (set `self.can interact` true))

(event `self.Sphere.OnComponentBeginOverlap`
  (params (OverlappedComponent :type "PrimitiveComponent Object Reference") (OtherActor :type "Actor Object Reference") (OtherComp :type "PrimitiveComponent Object Reference") (OtherBodyIndex :type Integer) (bFromSweep :type Boolean) (SweepResult :type "HitResult Structure (by ref)"))
  (if (== OtherActor (`GameplayStatics.GetPlayerPawn` 0))
    (if (`self.can interact`)
      (bind _returnvalue (`GameplayStatics.GetActorOfClass` "/Game/Blueprints/AAAAAAAAAAAAAAAA.AAAAAAAAAAAAAAAA_C"))
      (`/Game/Blueprints/AAAAAAAAAAAAAAAA.Add Bonus Pickup` _returnvalue (`self.pickup`))
      (bind (_direction _newtrack_0) (`Timeline|timeline effect bomb pickup` :!via `PlayFromStart`)
        (:`Update`
          (`SceneComponent.SetRelativeScale3D` (`self.StaticMesh`) (* _newtrack_0 (2.0 2.0 2.0))))
        (:`Finished`
          (`self.cool down`))))))

(event `cool down`
  (set `self.can interact` false)
  (`self.SetActorHiddenInGame` true)
  (`KismetSystemLibrary.Delay` 8.0)
  (`SceneComponent.SetRelativeScale3D` (`self.StaticMesh`) (2.0 2.0 2.0))
  (`self.SetActorHiddenInGame` false)
  (set `self.can interact` true))

(fn `UserConstructionScript`
  (bind _staticmesh (`self.StaticMesh`))
  (`SceneComponent.SetRelativeScale3D` (`self.Sphere`) (* (`self.collision size`) (1.0 1.0 1.0)))
  (switch `int` (`self.pickup`)
    (:`1`
      (`StaticMeshComponent.SetStaticMesh` _staticmesh "/Game/01_Meshes/cleaning_Product/SM_Produit_3.SM_Produit_3"))
    (:`2`
      (`StaticMeshComponent.SetStaticMesh` _staticmesh "/Game/01_Meshes/cleaning_Product/SM_Produit_1.SM_Produit_1"))
    (:`3`
      (`StaticMeshComponent.SetStaticMesh` _staticmesh "/Game/01_Meshes/cleaning_Product/SM_Produit_4.SM_Produit_4"))))