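; Nuke part pickup that the player collects by walking into its sphere trigger.
; The construction script scales the trigger by CollisionSize and selects one of four nuke meshes from NukePart.
; On player overlap, it calls AddNukePickup on the AAAAAAAAAAAAAAAA actor found in the level, then plays a timeline that animates the mesh scale and destroys the pickup when finished.
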(event `self.ReceiveBeginPlay`)

(event `self.Sphere.OnComponentBeginOverlap`
  (params (OverlappedComponent :type "PrimitiveComponent Object Reference") (OtherActor :type "Actor Object Reference") (OtherComp :type "PrimitiveComponent Object Reference") (OtherBodyIndex :type Integer) (bFromSweep :type Boolean) (SweepResult :type "HitResult Structure (by ref)"))
  (if (== OtherActor (`GameplayStatics.GetPlayerPawn` 0))
    (bind _returnvalue (`GameplayStatics.GetActorOfClass` "/Game/Blueprints/AAAAAAAAAAAAAAAA.AAAAAAAAAAAAAAAA_C"))
    (`/Game/Blueprints/AAAAAAAAAAAAAAAA.Add Nuke Pickup` _returnvalue)
    (bind (_direction _newtrack_0) (`Timeline|timeline effect bomb pickup` :!via `PlayFromStart`)
      (:`Update`
        (`SceneComponent.SetRelativeScale3D` (`self.StaticMesh`) (* _newtrack_0 (1.0 1.0 1.0))))
      (:`Finished`
        (`self.K2_DestroyActor`)))))

(fn `UserConstructionScript`
  (bind _staticmesh (`self.StaticMesh`))
  (`SceneComponent.SetRelativeScale3D` (`self.Sphere`) (* (`self.collision size`) (1.0 1.0 1.0)))
  (switch `int` (`self.nuke part`)
    (:`1`
      (`StaticMeshComponent.SetStaticMesh` _staticmesh "/Game/01_Meshes/SM_Nuke_01.SM_Nuke_01"))
    (:`2`
      (`StaticMeshComponent.SetStaticMesh` _staticmesh "/Game/01_Meshes/SM_Nuke_02.SM_Nuke_02"))
    (:`3`
      (`StaticMeshComponent.SetStaticMesh` _staticmesh "/Game/01_Meshes/SM_Nuke_03.SM_Nuke_03"))
    (:`4`
      (`StaticMeshComponent.SetStaticMesh` _staticmesh "/Game/01_Meshes/SM_Nuke_04.SM_Nuke_04"))))