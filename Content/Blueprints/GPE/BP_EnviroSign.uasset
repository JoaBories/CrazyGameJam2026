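; BP_EnviroSign is an environment sign actor with a Geometry Cache animation that starts when the player enters its overlap area.
; The construction script assigns the GeomCache asset to the component, and BeginPlay sets its Running flag to false.
; Overlap by player pawn 0 sets Running to true through SwitchAnim, with no end-overlap handler to reset it.
; Visibility-swap nodes are present but never run.
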(event `self.ReceiveBeginPlay`
  (`self.SwitchAnim` false))

(event `self.ReceiveActorBeginOverlap`
  (params (OtherActor :type "Actor Object Reference"))
  (if (== OtherActor (`GameplayStatics.GetPlayerPawn` 0))
    (`self.SwitchAnim` true)))

(event `SwitchAnim`
  (params (Anim :type Boolean))
  (set `GeometryCacheComponent.bRunning` Anim (`self.GeometryCache`)))

(fn `UserConstructionScript`
  (`GeometryCacheComponent.SetGeometryCache` (`self.GeometryCache`) (`self.GeomCache`)))