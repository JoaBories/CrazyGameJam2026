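; Proximity-reactive light actor that changes the colour of its sphere as the player pawn approaches or leaves.
; Nested near and far trigger spheres, scaled from distance variables in the construction script, select the near colour, the far colour, or zero values outside both.
; Colours are written as default custom primitive data on the sphere, so its material can read them without dynamic material instances.
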(event `self.Sphere_near.OnComponentBeginOverlap`
  (params (OverlappedComponent :type "PrimitiveComponent Object Reference") (OtherActor :type "Actor Object Reference") (OtherComp :type "PrimitiveComponent Object Reference") (OtherBodyIndex :type Integer) (bFromSweep :type Boolean) (SweepResult :type "HitResult Structure (by ref)"))
  (bind (_colour_near_b _colour_near_g _colour_near_r _colour_near_a) (break `Color` (`self.colour_Near`)))
  (if (== OtherActor (`GameplayStatics.GetPlayerPawn` 0))
    (`PrimitiveComponent.SetDefaultCustomPrimitiveDataVector4` (`self.Sphere`) 0 (`KismetMathLibrary.MakeVector4` (`KismetMathLibrary.Conv_ByteToDouble` _colour_near_r) (`KismetMathLibrary.Conv_ByteToDouble` _colour_near_g) (`KismetMathLibrary.Conv_ByteToDouble` _colour_near_b) (`KismetMathLibrary.Conv_ByteToDouble` _colour_near_a)))))

(event `self.Sphere_near.OnComponentEndOverlap`
  (params (OverlappedComponent :type "PrimitiveComponent Object Reference") (OtherActor :type "Actor Object Reference") (OtherComp :type "PrimitiveComponent Object Reference") (OtherBodyIndex :type Integer))
  (bind (_b _g _r _a) (break `Color` (`self.colour_Far`)))
  (if (== OtherActor (`GameplayStatics.GetPlayerPawn` 0))
    (`PrimitiveComponent.SetDefaultCustomPrimitiveDataVector4` (`self.Sphere`) 0 (`KismetMathLibrary.MakeVector4` (`KismetMathLibrary.Conv_ByteToDouble` _r) (`KismetMathLibrary.Conv_ByteToDouble` _g) (`KismetMathLibrary.Conv_ByteToDouble` _b) (`KismetMathLibrary.Conv_ByteToDouble` _a)) :!label _label)))

(event `self.Sphere_far.OnComponentBeginOverlap`
  (params (OverlappedComponent :type "PrimitiveComponent Object Reference") (OtherActor :type "Actor Object Reference") (OtherComp :type "PrimitiveComponent Object Reference") (OtherBodyIndex :type Integer) (bFromSweep :type Boolean) (SweepResult :type "HitResult Structure (by ref)"))
  (if (== OtherActor (`GameplayStatics.GetPlayerPawn` 0))
    (goto _label)))

(event `self.Sphere_far.OnComponentEndOverlap`
  (params (OverlappedComponent :type "PrimitiveComponent Object Reference") (OtherActor :type "Actor Object Reference") (OtherComp :type "PrimitiveComponent Object Reference") (OtherBodyIndex :type Integer))
  (if (== OtherActor (`GameplayStatics.GetPlayerPawn` 0))
    (`PrimitiveComponent.SetDefaultCustomPrimitiveDataVector4` (`self.Sphere`) 0 (0.0 0.0 0.0 0.0))))

(fn `UserConstructionScript`
  (bind _returnvalue (`KismetMathLibrary.Conv_IntToDouble` (`self.Far_Distance`)))
  (bind _returnvalue_2 (`KismetMathLibrary.Conv_IntToDouble` (`self.Near_Distance`)))
  (`SceneComponent.SetRelativeScale3D` (`self.Sphere_near`) (`KismetMathLibrary.MakeVector` _returnvalue_2 _returnvalue_2 _returnvalue_2))
  (`SceneComponent.SetRelativeScale3D` (`self.Sphere_far`) (`KismetMathLibrary.MakeVector` _returnvalue _returnvalue _returnvalue)))