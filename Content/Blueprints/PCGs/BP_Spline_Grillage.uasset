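; Spline-driven fence (grillage) actor that rebuilds itself along its spline in the construction script.
; It steps the spline at DistanceBetweenVertical intervals, placing HISM instances midway between points, oriented along each segment, with separate static mesh components at start and end.
; The first segment gets no instance.
; Segment pieces get slight position and rotation jitter from a random stream seeded by actor location.
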(fn `create fence`
  (locals (`distance between vertical` :type "Float (double-precision)" :default 300.0) (`current index` :type Integer) (stream :type "RandomStream Structure"))
  (bind _spline (`self.Spline`))
  (bind _current_index (`local.current index`))
  (bind _distance_between_vertical (`local.distance between vertical`))
  (bind _returnvalue (`KismetMathLibrary.RandomFloatInRangeFromStream` (`local.stream`) -0.5 0.5))
  (bind _returnvalue_2 (`SplineComponent.GetLocationAtDistanceAlongSpline` (`self.Spline`) (* (`local.distance between vertical`) _current_index) "Local"))
  (bind _returnvalue_3 (`KismetMathLibrary.FTrunc` (/ (`SplineComponent.GetSplineLength` (`self.Spline`)) _distance_between_vertical)))
  (bind _returnvalue_4 (`SplineComponent.GetLocationAtDistanceAlongSpline` (`self.Spline`) (* (`local.distance between vertical`) (- _current_index 1)) "Local"))
  (bind _returnvalue_5 (`KismetMathLibrary.MakeTransform` (+ (`KismetMathLibrary.VLerp` _returnvalue_4 _returnvalue_2 0.5) (`KismetMathLibrary.MakeVector` 0.0 (`KismetMathLibrary.RandomFloatInRangeFromStream` (`local.stream`) -5.0 5.0) (`KismetMathLibrary.RandomFloatInRangeFromStream` (`local.stream`) -10.0 10.0))) (`KismetMathLibrary.MakeRotator` (+ (.roll (`KismetMathLibrary.FindLookAtRotation` _returnvalue_4 _returnvalue_2)) _returnvalue) (+ (.pitch (`KismetMathLibrary.FindLookAtRotation` _returnvalue_4 _returnvalue_2)) (`KismetMathLibrary.RandomFloatInRangeFromStream` (`local.stream`) -1.0 1.0)) (+ (.yaw (`KismetMathLibrary.FindLookAtRotation` _returnvalue_4 _returnvalue_2)) _returnvalue))))
  (set `local.stream` (`KismetMathLibrary.MakeRandomStreamFromLocation` (`SceneComponent.K2_GetComponentLocation` (`self.DefaultSceneRoot`)) 300.0))
  (bind _returnvalue_6 (* _distance_between_vertical (stale _index)))
  (`AddComponent|NODE_AddStaticMeshComponent-0` :`RelativeTransform` (`KismetMathLibrary.MakeTransform` (`SplineComponent.GetLocationAtDistanceAlongSpline` _spline _returnvalue_6 "Local") (`KismetMathLibrary.Conv_VectorToRotator` (`SplineComponent.GetTangentAtDistanceAlongSpline` _spline _returnvalue_6 "Local"))))
  (for _index (range (+ _returnvalue_3 1))
    (bind _output_get (set `local.current index` _index))
    (if (!= _output_get 1)
      (if (!= _current_index _returnvalue_3)
        (if (!= (`local.current index`) 0)
          (`InstancedStaticMeshComponent.AddInstance` (`self.HISM_Fence`) _returnvalue_5 false))
        (else
          (`AddComponent|NODE_AddStaticMeshComponent-2` :`RelativeTransform` _returnvalue_5))))))

(fn `UserConstructionScript`
  (`self.create fence`))