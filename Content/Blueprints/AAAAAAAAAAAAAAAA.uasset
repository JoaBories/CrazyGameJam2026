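; Player pawn, apparently a shopping cart, driven as a physics sphere with an orbit camera.
; Grounded move input adds camera-relative torque, using velocity-to-input dot products for braking and drift effects.
; A per-tick sphere trace detects ground; airborne input triggers timeline-driven mesh rotation tricks with trails and escalating combo sounds.
; It also handles pause, bonus counts, attack cycling (firing is empty), game over, and an end cinematic after four nuke parts.
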(event `Tricks Left`
  (set `self.Currently Tricksmaxxing` true)
  (`self.Play trick Sound`)
  (bind (_direction _rotation) (`Timeline|Rot` :!via `PlayFromStart`)
    (:`Update`
      (`SceneComponent.K2_SetRelativeRotation` (`self.Cube`) (`KismetMathLibrary.MakeRotator` _rotation) false false))
    (:`Finished`
      (set `self.Currently Tricksmaxxing` false))))

(event `Play trick Sound`
  (`|ExecutionSequence`
    (:`then_0`
      (`ActorComponent.Activate` (`self.NS_TrickTrails`) false)
      (`ActorComponent.Activate` (`self.NS_TrickTrails1`) false)
      (`GameplayStatics.PlaySound2D` (select `int` (`KismetMathLibrary.Clamp` (`self.Trick Int`) 0 7) :`0` "/Game/Developers/Alex/Jet_Set_Radio_-_All_Spray_Sound_Effects__HQ___mp3cut_net_.Jet_Set_Radio_-_All_Spray_Sound_Effects__HQ___mp3cut_net_" :`1` "/Game/Developers/Alex/Jet_Set_Radio_-_All_Spray_Sound_Effects__HQ___mp3cut_net__1_.Jet_Set_Radio_-_All_Spray_Sound_Effects__HQ___mp3cut_net__1_" :`2` "/Game/Developers/Alex/Jet_Set_Radio_-_All_Spray_Sound_Effects__HQ___mp3cut_net__2_.Jet_Set_Radio_-_All_Spray_Sound_Effects__HQ___mp3cut_net__2_" :`3` "/Game/Developers/Alex/Jet_Set_Radio_-_All_Spray_Sound_Effects__HQ___mp3cut_net__3_.Jet_Set_Radio_-_All_Spray_Sound_Effects__HQ___mp3cut_net__3_" :`4` "/Game/Developers/Alex/Jet_Set_Radio_-_All_Spray_Sound_Effects__HQ___mp3cut_net__4_.Jet_Set_Radio_-_All_Spray_Sound_Effects__HQ___mp3cut_net__4_" :`5` "/Game/Developers/Alex/Jet_Set_Radio_-_All_Spray_Sound_Effects__HQ___mp3cut_net__5_.Jet_Set_Radio_-_All_Spray_Sound_Effects__HQ___mp3cut_net__5_" :`6` "/Game/Developers/Alex/Jet_Set_Radio_-_All_Spray_Sound_Effects__HQ___mp3cut_net__6_.Jet_Set_Radio_-_All_Spray_Sound_Effects__HQ___mp3cut_net__6_" :`7` "/Game/Developers/Alex/Jet_Set_Radio_-_All_Spray_Sound_Effects__HQ___mp3cut_net__7_.Jet_Set_Radio_-_All_Spray_Sound_Effects__HQ___mp3cut_net__7_" :!type "SoundBase Object Reference") 1.0 1.0 0.0 null null)
      (`/Engine/EditorBlueprintResources/StandardMacros.IncrementInt` (`self.Trick Int`)))
    (:`then_1`
      (`KismetSystemLibrary.RetriggerableDelay` 1.0)
      (set `self.Trick Int` 0)
      (`ActorComponent.Deactivate` (`self.NS_TrickTrails`))
      (`ActorComponent.Deactivate` (`self.NS_TrickTrails1`)))))

(event `Tricks Right`
  (set `self.Currently Tricksmaxxing` true)
  (`self.Play trick Sound`)
  (bind (_direction _rotation) (`Timeline|Timeline` :!via `PlayFromStart`)
    (:`Update`
      (`SceneComponent.K2_SetRelativeRotation` (`self.Cube`) (`KismetMathLibrary.MakeRotator` (* _rotation -1.0)) false false))
    (:`Finished`
      (set `self.Currently Tricksmaxxing` false))))

(event `Tricks Up`
  (set `self.Currently Tricksmaxxing` true)
  (`self.Play trick Sound`)
  (bind (_direction _rotation) (`Timeline|Timeline_0` :!via `PlayFromStart`)
    (:`Update`
      (`SceneComponent.K2_SetRelativeRotation` (`self.Cube`) (`KismetMathLibrary.MakeRotator` 0.0 _rotation) false false))
    (:`Finished`
      (set `self.Currently Tricksmaxxing` false))))

(event `Tricks Down`
  (set `self.Currently Tricksmaxxing` true)
  (`self.Play trick Sound`)
  (bind (_direction _rotation) (`Timeline|Timeline_1` :!via `PlayFromStart`)
    (:`Update`
      (`SceneComponent.K2_SetRelativeRotation` (`self.Cube`) (`KismetMathLibrary.MakeRotator` 0.0 (* _rotation -1.0)) false false))
    (:`Finished`
      (set `self.Currently Tricksmaxxing` false))))

(event `Add Bonus Pickup`
  (params (`Pickup Int` :type Integer))
  (`/Engine/EditorBlueprintResources/StandardMacros.IncrementInt` (`|GetArrayItem` (`self.Bonuses`) `Pickup Int`)))

(event `Add Nuke Pickup`
  (bind _nuke_part (`self.Nuke Part`))
  (`/Engine/EditorBlueprintResources/StandardMacros.IncrementInt` _nuke_part
    (:`  `
      (if (== _nuke_part 4)
        (bind _returnvalue (`|CreateWidget` "/Game/Cinematic/WBP_end_cinematic.WBP_end_cinematic_C" (`GameplayStatics.GetPlayerController` 0)))
        (`UserWidget.AddToViewport` _returnvalue 0)
        (`self.K2_AddActorWorldOffset` (0.0 0.0 -1000.0))))))

(event `Take Damage`
  (bind _result (`/Engine/EditorBlueprintResources/StandardMacros.DecrementInt` (`self.Life`))
    (:`  `
      (if (< _result 0)
        (bind _returnvalue (`|CreateWidget` "/Game/Menus/Viewport/WBP_GameOver.WBP_GameOver_C" (`GameplayStatics.GetPlayerController` 0)))
        (`UserWidget.AddToViewport` _returnvalue 0)))))

(event `self.ReceiveBeginPlay`
  (bind _returnvalue (`|CreateWidget` "/Game/Developers/Alex/WBP_CyrianShoppingCartPlayerDebugInfos.WBP_CyrianShoppingCartPlayerDebugInfos_C" (`GameplayStatics.GetPlayerController` 0)))
  (bind _output_get (set `self.Debug Widget` _returnvalue))
  (`UserWidget.AddToViewport` _output_get 0)
  (set `self.Bonuses` (`|MakeArray` 0 0 0)))

(event `self.ReceiveTick`
  (params (DeltaSeconds :type "Float (single-precision)"))
  (bind _returnvalue (`SceneComponent.GetComponentVelocity` (`self.Sphere`)))
  (bind _returnvalue_2 (`SceneComponent.K2_GetComponentLocation` (`self.Sphere`)))
  (`SceneComponent.K2_SetWorldLocation` (`self.AAAA`) (`SceneComponent.K2_GetComponentLocation` (`self.Sphere`)) false false)
  (bind (_outhit _returnvalue_3) (`KismetSystemLibrary.SphereTraceSingle` :`Start` _returnvalue_2 :`End` _returnvalue_2 :`Radius` 53.0 :`TraceChannel` "TraceTypeQuery1" :`DrawDebugType` "ForOneFrame"))
  (set `self.is Grounded` _returnvalue_3)
  (`/Game/Developers/Alex/WBP_CyrianShoppingCartPlayerDebugInfos.Set Kilometer` (`self.Debug Widget`) (`KismetMathLibrary.FTrunc` (`KismetMathLibrary.VSize` (`SceneComponent.GetComponentVelocity` (`self.Sphere`)))))
  (if (!= _returnvalue (0.0 0.0 0.0) :`ErrorTolerance` 10.0)
    (`SceneComponent.K2_SetWorldRotation` (`self.Scene1`) (`KismetMathLibrary.FindLookAtRotation` (`KismetMathLibrary.MakeVector` 0.0) (`KismetMathLibrary.Normal` _returnvalue)) false false)))

(event `EnhancedInput|/Game/Input/Actions/IA_Move`
  (params (ActionValue :type "Vector2D Structure") (ElapsedSeconds :type "Float (double-precision)") (TriggeredSeconds :type "Float (double-precision)") (InputAction :type "InputAction Object Reference" :default "/Game/Input/Actions/IA_Move.IA_Move"))
  (bind _returnvalue (`KismetMathLibrary.Abs` ActionValue_Y))
  (bind _returnvalue_2 (`KismetMathLibrary.Abs` ActionValue_X))
  (bind _sphere (`self.Sphere`))
  (bind _sphere_2 (`self.Sphere`))
  (bind _ns_drifting (`self.NS_Drifting`))
  (bind _ns_drifting1 (`self.NS_Drifting1`))
  (bind _returnvalue_3 (`SceneComponent.GetComponentVelocity` _sphere_2))
  (bind (_returnvalue_x _returnvalue_y) (`KismetMathLibrary.BreakVector` (`SceneComponent.GetComponentVelocity` _sphere)))
  (bind _returnvalue_4 (`ActorComponent.IsActive` (`self.NS_Drifting`)))
  (bind _returnvalue_5 (`KismetMathLibrary.Normal` (`KismetMathLibrary.ProjectVectorOnToPlane` (+ (* (`SceneComponent.GetForwardVector` (`self.Camera`)) ActionValue_X -1.0) (* (`SceneComponent.GetRightVector` (`self.Camera`)) ActionValue_Y)) (0.0 0.0 1.0))))
  (bind (_returnvalue_x_2 _returnvalue_y_2) (`KismetMathLibrary.BreakVector` (* _returnvalue_5 (`self.Acceleration Speed`) (`GameplayStatics.GetWorldDeltaSeconds`))))
  (bind _returnvalue_6 (`KismetMathLibrary.Dot_VectorVector` (`KismetMathLibrary.Normal` (`KismetMathLibrary.MakeVector` _returnvalue_x _returnvalue_y)) (`KismetMathLibrary.Normal` (`KismetMathLibrary.MakeVector` (.y _returnvalue_5) (* (.x _returnvalue_5) -1.0)))))
  (:`Triggered`
    (if (`self.is Grounded`)
      (if (>= _returnvalue_6 -0.25)
        (`PrimitiveComponent.AddTorqueInRadians` _sphere (`KismetMathLibrary.MakeVector` _returnvalue_x_2 _returnvalue_y_2) "None" true)
        (if (>= _returnvalue_6 0.33)
          (if _returnvalue_4
            (`ActorComponent.Deactivate` _ns_drifting)
            (`ActorComponent.Deactivate` _ns_drifting1))
          (elif (not _returnvalue_4)
            (`ActorComponent.Activate` _ns_drifting false)
            (`ActorComponent.Activate` _ns_drifting1 false)))
        (elif (`self.is Grounded`)
          (`PrimitiveComponent.SetPhysicsLinearVelocity` _sphere_2 (- _returnvalue_3 (* _returnvalue_3 (`self.Brake Speed`) (`GameplayStatics.GetWorldDeltaSeconds`))) false "None")
          (`PrimitiveComponent.AddTorqueInRadians` _sphere_2 (`KismetMathLibrary.MakeVector` _returnvalue_x_2 _returnvalue_y_2) "None" true)))
      (elif (and (not (`self.Currently Tricksmaxxing`)) (< (`KismetMathLibrary.FMax` _returnvalue_2 _returnvalue) 0.6))
        (if (> _returnvalue_2 _returnvalue)
          (if (> ActionValue_X 0.0)
            (`self.Tricks Left`)
            (else
              (`self.Tricks Right`)))
          (elif (> ActionValue_Y 0.0)
            (`self.Tricks Up`)
            (else
              (`self.Tricks Down`)))))))
  (:`Canceled`
    (`PrimitiveComponent.SetAngularDamping` (`self.Sphere`) 10.0 :!label _label))
  (:`Completed`
    (goto _label)))

(event `EnhancedInput|/Game/Input/Actions/IA_Look`
  (params (ActionValue :type "Vector2D Structure") (ElapsedSeconds :type "Float (double-precision)") (TriggeredSeconds :type "Float (double-precision)") (InputAction :type "InputAction Object Reference" :default "/Game/Input/Actions/IA_Look.IA_Look"))
  (bind _springarm (`self.SpringArm`))
  (bind _camera_turning_speed (`self.Camera Turning Speed`))
  (bind (_relativerotation_roll _relativerotation_pitch _relativerotation_yaw) (`KismetMathLibrary.BreakRotator` (`SceneComponent.RelativeRotation` _springarm)))
  (:`Triggered`
    (`SceneComponent.K2_AddRelativeRotation` (`self.SpringArm`) (`KismetMathLibrary.MakeRotator` 0.0 (* (* ActionValue_Y -1.0) _camera_turning_speed) (* ActionValue_X _camera_turning_speed)) false false)
    (`SceneComponent.K2_SetRelativeRotation` _springarm (`KismetMathLibrary.MakeRotator` _relativerotation_roll (`KismetMathLibrary.FClamp` _relativerotation_pitch -85.0 -10.0) _relativerotation_yaw) false false)))

(event `EnhancedInput|/Game/Input/Actions/IA_Pause`
  (params (ActionValue :type "Vector2D Structure") (ElapsedSeconds :type "Float (double-precision)") (TriggeredSeconds :type "Float (double-precision)") (InputAction :type "InputAction Object Reference" :default "/Game/Input/Actions/IA_Pause.IA_Pause"))
  (bind _returnvalue (`GameplayStatics.GetPlayerController` 0))
  (bind _returnvalue_2 (`GameplayStatics.GetPlayerController` 0))
  (bind _pause_ref (`self.Pause Ref`))
  (:`Triggered`
    (`/Engine/EditorBlueprintResources/StandardMacros.IsValid` (`self.Pause Ref`)
      (:`Is Valid`
        _)
      (:`Is Not Valid`
        (bind _returnvalue_3 (`|CreateWidget` "/Game/Menus/Viewport/WBP_PauseMenu.WBP_PauseMenu_C"))
        (set `self.Pause Ref` _returnvalue_3)))
    (if (`GameplayStatics.IsGamePaused`)
      (`Widget.RemoveFromParent` (`self.Pause Ref`))
      (`GameplayStatics.SetGamePaused` false)
      (set `PlayerController.bShowMouseCursor` false _returnvalue_2)
      (`WidgetBlueprintLibrary.SetInputMode_GameOnly` _returnvalue_2)
      (else
        (`UserWidget.AddToViewport` _pause_ref 0)
        (`GameplayStatics.SetGamePaused` true)
        (set `PlayerController.bShowMouseCursor` true _returnvalue)
        (`WidgetBlueprintLibrary.SetInputMode_UIOnlyEx` _returnvalue null)
        (`Widget.SetKeyboardFocus` (`/Game/Menus/Viewport/WBP_PauseMenu.ResumeButton` _pause_ref))))))

(event `EnhancedInput|/Game/Input/Actions/IA_Attack`
  (params (ActionValue :type "Vector2D Structure") (ElapsedSeconds :type "Float (double-precision)") (TriggeredSeconds :type "Float (double-precision)") (InputAction :type "InputAction Object Reference" :default "/Game/Input/Actions/IA_Attack.IA_Attack")))

(event `EnhancedInput|/Game/Input/Actions/IA_ChangeAttack`
  (params (ActionValue :type "Float (double-precision)") (ElapsedSeconds :type "Float (double-precision)") (TriggeredSeconds :type "Float (double-precision)") (InputAction :type "InputAction Object Reference" :default "/Game/Input/Actions/IA_ChangeAttack.IA_ChangeAttack"))
  (bind _currentattack (`self.CurrentAttack`))
  (:`Started`
    (if (> ActionValue 0.0)
      (bind _result (`/Engine/EditorBlueprintResources/StandardMacros.IncrementInt` _currentattack)
        (:`  `
          (if (> _result 2)
            (set `self.CurrentAttack` 0))))
      (else
        (bind _result_2 (`/Engine/EditorBlueprintResources/StandardMacros.DecrementInt` _currentattack)
          (:`  `
            (if (< _result_2 0)
              (set `self.CurrentAttack` 2))))))))

(fn `UserConstructionScript`)