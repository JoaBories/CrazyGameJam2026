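; Help is a trigger actor that redirects and caps the velocity of an AAAAAAAAAAAAAAAA actor's physics Sphere on overlap.
; It acts only when the Sphere's vertical velocity is zero or upward.
; The velocity is projected onto the plane normal to the Arrow's forward vector, removing motion along that axis.
; X and Y are then clamped to ±MaxSideVel and Z between zero and MaxZVel.
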(event `self.ReceiveActorBeginOverlap`
  (params (OtherActor :type "Actor Object Reference"))
  (bind _max_side_vel (`self.Max Side Vel`))
  (bind _returnvalue (* _max_side_vel -1.0))
  (bind _asaaaaaaaaaaaaaaaa (cast `/Game/Blueprints/AAAAAAAAAAAAAAAA` OtherActor))
  (bind _sphere (`/Game/Blueprints/AAAAAAAAAAAAAAAA.Sphere` _asaaaaaaaaaaaaaaaa))
  (bind _returnvalue_2 (`SceneComponent.GetComponentVelocity` _sphere))
  (if (>= (.z _returnvalue_2) 0.0)
    (bind (_returnvalue_x _returnvalue_y _returnvalue_z) (`KismetMathLibrary.BreakVector` (`KismetMathLibrary.ProjectVectorOnToPlane` _returnvalue_2 (`SceneComponent.GetForwardVector` (`self.Arrow`)))))
    (`PrimitiveComponent.SetPhysicsLinearVelocity` _sphere (`KismetMathLibrary.MakeVector` (`KismetMathLibrary.FClamp` _returnvalue_x _returnvalue _max_side_vel) (`KismetMathLibrary.FClamp` _returnvalue_y _returnvalue _max_side_vel) (`KismetMathLibrary.FClamp` _returnvalue_z 0.0 (`self.Max Z Vel`))) false "None")))

(fn `UserConstructionScript`)